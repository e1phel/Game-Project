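; Melee enemy character that patrols waypoints in a loop and chases the player once seen.
; PawnSensing raises walk speed, plays a one-time alert and starts an AIMoveTo chase, which on arrival fires flag-gated cross and jab montages.
; Punch hitbox overlaps only print debug text.
; Capsule overlaps tagged "Hit" play a reaction and decrement HP, with a death montage, collision shutoff and delayed destroy at zero.
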(event OnSeePawn(PawnSensing)
  (params (Pawn :type Pawn%20Object%20Reference))
  (CallFunction|ChasePlayer)
  (Variables|/Script/Engine.CharacterMovementComponent|SetMaxWalkSpeed (Variables|Character|GetCharacterMovement) 5.5e+02)
  (if (Variables|Default|Getsound)
    (Audio|PlaySound2D "/Game/sounds/Alert.Alert" 1.0 1.0 0.0 0 0)
    (Variables|Default|Setsound false)))

(event OnComponentBeginOverlap(CapsuleComponent)
  (params (OverlappedComponent :type Primitive%20Component%20Object%20Reference) (OtherActor :type Actor%20Object%20Reference) (OtherComp :type Primitive%20Component%20Object%20Reference) (OtherBodyIndex :type Integer) (bFromSweep :type Boolean) (SweepResult :type Hit%20Result%20Structure%20%28by%20ref%29))
  (if (Components|ComponentHasTag OtherComp "Hit")
    (Animation|Montage|PlayMontage (Variables|Character|GetMesh) "/Game/Characters/Rogue_Character_Model-15e2afd1/fbx/AL_Standard_Anim_Rig_Hit_Chest_Montage.AL_Standard_Anim_Rig_Hit_Chest_Montage"
      (:then
        (Development|PrintText "HIt_done" true true "(R=1.000000,G=0.000000,B=0.104368,A=1.000000)")
        (if (> (Variables|Default|GetHP) 0)
          (Development|PrintString "-HP" true true "(R=0.482292,G=0.043686,B=0.000000,A=1.000000)")
          (Math|Integer|DecrementInt (Variables|Default|GetHP)
            (:%20%20
              (CallFunction|Death))))))))

(event OnComponentBeginOverlap(Hit_detect)
  (params (OverlappedComponent :type Primitive%20Component%20Object%20Reference) (OtherActor :type Actor%20Object%20Reference) (OtherComp :type Primitive%20Component%20Object%20Reference) (OtherBodyIndex :type Integer) (bFromSweep :type Boolean) (SweepResult :type Hit%20Result%20Structure%20%28by%20ref%29))
  (if (Components|ComponentHasTag OtherComp "Player")
    (Development|PrintText "Hit")))

(event OnComponentBeginOverlap(Hit_detect1)
  (params (OverlappedComponent :type Primitive%20Component%20Object%20Reference) (OtherActor :type Actor%20Object%20Reference) (OtherComp :type Primitive%20Component%20Object%20Reference) (OtherBodyIndex :type Integer) (bFromSweep :type Boolean) (SweepResult :type Hit%20Result%20Structure%20%28by%20ref%29))
  (if (Components|ComponentHasTag OtherComp "Player")
    (Development|PrintText "Follow Up")))

(event Custom|Move
  (bind _waypoint (Variables|Default|GetWaypoint))
  (AI|AIMoveTo self "0, 0, 0" (Utilities|Array|Get(acopy) _waypoint (Variables|Default|Getindex)) 5.0 false
    (:OnSuccess
      (bind _result (Math|Integer|IncrementInt (Variables|Default|Getindex))
        (:%20%20
          (if (>= (Variables|Default|Getindex) (Utilities|Array|Length _waypoint))
            (Variables|Default|Setindex 0)
            (else
              (Variables|Default|Setindex _result)))
          (CallFunction|Move self)
          (Variables|/Script/Engine.CharacterMovementComponent|SetMaxWalkSpeed (Variables|Character|GetCharacterMovement) 2.2e+02))))))

(event Custom|Chase%20Player
  (AI|AIMoveTo self "0, 0, 0" (Game|GetPlayerCharacter 0) 5.0 false
    (:OnSuccess
      (if (Variables|Default|Getallow_atk)
        (Animation|Montage|PlayMontage (Variables|Character|GetMesh) "/Game/Characters/Rogue_Character_Model-15e2afd1/fbx/AL_Standard_Anim_Rig_Punch_Cross_Montage.AL_Standard_Anim_Rig_Punch_Cross_Montage"
          (:then
            (Variables|Default|Setallow_atk false)
            (if (Variables|Default|Getatk_done)
              (Animation|Montage|PlayMontage (Variables|Character|GetMesh) "/Game/Characters/Rogue_Character_Model-15e2afd1/fbx/AL_Standard_Anim_Rig_Punch_Jab_Montage.AL_Standard_Anim_Rig_Punch_Jab_Montage"
                (:then
                  (Variables|Default|Setatk_done false))
                (:OnCompleted
                  (Variables|Default|Setatk_done true :!label _label))
                (:OnInterrupted
                  (goto _label)))))
          (:OnCompleted
            (Variables|Default|Setallow_atk true :!label _label_2))
          (:OnInterrupted
            (goto _label_2)))))))

(event Custom|check_dead
  (if (Variables|Default|GetDead)
    (Actor|DestroyActor)))

(event Custom|Death
  (if (<= (Variables|Default|GetHP) 0)
    (Animation|Montage|PlayMontage (Variables|Character|GetMesh) "/Game/Characters/Rogue_Character_Model-15e2afd1/fbx/AL_Standard_Anim_Rig_Death01_Montage.AL_Standard_Anim_Rig_Death01_Montage"
      (:then
        (Collision|SetCollisionEnabled (Variables|Collision|GetCapsuleComponent) "NoCollision")
        (Utilities|FlowControl|Delay 2.2)
        (Actor|DestroyActor)))))

(event EventBeginPlay
  (CallFunction|Move))

(fn ConstructionScript)